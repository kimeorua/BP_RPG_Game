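; Base character Blueprint that resolves incoming melee-style damage into guard, parry, hit or death reactions.
; AnyDamage lets frontal attacks be blocked or countered when state and damage type match; otherwise HP drops and data-asset montages play directional hit or random death reactions.
; Guarding drains own SP until guard break, while a timed guard parry drains the attacker's SP, staggering them and refilling it at zero.
; Counter parry staggers the attacker directly.
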(event EventBeginPlay
  (Variables|/Game/BP/Component/BP_StateComponent.BP_StateComponent_C|SetMy%20State (Variables|Default|GetStateComponent) "NewEnumerator1"))

(event EventTick
  (params (DeltaSeconds :type Float%20%28single-precision%29)))

(event Game|Damage|EventAnyDamage
  (params (Damage :type Float%20%28single-precision%29) (DamageType :type Damage%20Type%20Object%20Reference) (InstigatedBy :type Controller%20Object%20Reference) (DamageCauser :type Actor%20Object%20Reference))
  (if (CallFunction|CheackState DamageCauser)
    (switch Utilities|FlowControl|Switch|SwitchonE_State (Variables|/Game/BP/Component/BP_StateComponent.BP_StateComponent_C|GetMy%20State (Variables|Default|GetStateComponent))
      (:NewEnumerator4
        (if (== (Utilities|GetClass DamageType) "/Game/BP/EnumAndStruct/DamageType/BP_DamageType_GuardAble.BP_DamageType_GuardAble_C")
          (|Guard Damage DamageCauser)
          (else
            (CallFunction|HitandDie Damage DamageCauser :!label _label))))
      (:NewEnumerator9
        (if (== (Utilities|GetClass DamageType) "/Game/BP/EnumAndStruct/DamageType/BP_DamageType_OnlyParry.BP_DamageType_OnlyParry_C")
          (|Parry DamageCauser)
          (else
            (goto _label)))))
    (else
      (CallFunction|HitandDie Damage DamageCauser))))

(fn ConstructionScript)

(fn JumpAttackEnd
  (Variables|Combet|SetJumpAttack false)
  (Variables|/Game/BP/Component/BP_StateComponent.BP_StateComponent_C|SetMy%20State (Variables|Default|GetStateComponent) "NewEnumerator1"))

(fn CalculateHitDirection
  (params (Causer :type Actor%20Object%20Reference))
  (bind _hit_and_die_dataasset (Variables|Combet|GetHit%20And%20Die%20DataAsset))
  (bind _hitmontage (Variables|/Game/BP/DataAsset/Character_DataAsset/BP_HitAndDieDataAsset.BP_HitAndDieDataAsset_C|GetHitMontage _hit_and_die_dataasset))
  (bind _returnvalue (Utilities|Array|Length _hitmontage))
  (if (> _returnvalue 1)
    (LocalVariables|SetDegree (/ (LocalVariables|GetRotation) _returnvalue))
    (return (Math|Float|Truncate (/ (Math|Float|%(Float) (+ (Class|KismetAnimationLibrary|CalculateDirection (- (Transformation|GetActorLocation (Components|GetOwner Causer)) (Transformation|GetActorLocation)) (Math|Rotator|MakeRotator 0.0 0.0 (.yaw (Pawn|GetControlRotation :!class /Script/Engine.Pawn)))) 3.6e+02) 3.6e+02) (LocalVariables|GetDegree))))
    (else
      (return 0))))

(fn ResetParrAble
  (Variables|Combet|SetIsParryAble false))

(fn SPDawn
  (Default|ChangeStatus (Variables|Default|GetStatusComponent) "NewEnumerator3" (Variables|/Game/BP/DataAsset/Weapon_DataAsset/BP_WeaponData.BP_WeaponData_C|GetAttackSP (Variables|/Game/BP/Component/BP_WeaponComponent.BP_WeaponComponent_C|GetCurrent%20Weapon%20Data (Variables|Default|GetWeaponComponent))) 0.0))

(fn SelecteStatus
  (params (StatusType :type E_StatusType%20Enum :default "NewEnumerator2"))
  (bind _statuscomponent (Variables|Default|GetStatusComponent))
  (bind _currentstauts (Variables|/Game/BP/Component/BP_StatusComponent.BP_StatusComponent_C|GetCurrentStauts _statuscomponent))
  (bind (_hp _sp) (Utilities|Struct|BreakF_Status _currentstauts))
  (switch Utilities|FlowControl|Switch|SwitchonE_StatusType StatusType
    (:NewEnumerator0
      (return _hp))
    (:NewEnumerator3
      (return _sp))))

(fn CheackDirection
  (params (Causer :type Actor%20Object%20Reference))
  (bind _returnvalue (Components|GetOwner Causer))
  (bind _returnvalue_2 (Transformation|GetActorRotation))
  (bind _returnvalue_3 (Transformation|GetActorLocation))
  (bind _returnvalue_4 (Transformation|GetActorLocation _returnvalue))
  (bind _returnvalue_5 (- _returnvalue_4 _returnvalue_3))
  (bind _returnvalue_6 (Class|KismetAnimationLibrary|CalculateDirection _returnvalue_5 (Math|Rotator|MakeRotator 0.0 0.0 (.yaw _returnvalue_2))))
  (bind _returnvalue_7 (+ _returnvalue_6 3.6e+02))
  (bind _returnvalue_8 (Math|Float|%(Float) _returnvalue_7 3.6e+02))
  (return (or (<= _returnvalue_8 45.0) (>= _returnvalue_8 315.0))))

(fn CheackState
  (params (Causer :type Actor%20Object%20Reference))
  (bind _statecomponent (Variables|Default|GetStateComponent))
  (bind _my_state (Variables|/Game/BP/Component/BP_StateComponent.BP_StateComponent_C|GetMy%20State _statecomponent))
  (if (and (or (Utilities|Enum|Equal(Enum) _my_state "NewEnumerator9") (Utilities|Enum|Equal(Enum) _my_state "NewEnumerator4")) (CallFunction|CheackDirection Causer))
    (return true)
    (else
      (return false))))

(fn HitandDie
  (params (Damage :type Float%20%28double-precision%29) (Causer :type Actor%20Object%20Reference))
  (|HitAndDamage Damage Causer))
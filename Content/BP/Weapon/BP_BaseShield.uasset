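; BP_BaseShield is the base shield actor for a BP_BaseCharacter, providing attachment, highlight and counter-parry behavior.
; On BeginPlay it caches its owning character and replaces every mesh material with a dynamic instance.
; AttachShield parents a given component to a socket on the character mesh, while ColorOnOff toggles the first material's Color between bright tint and white.
; CounterParryActivate plays the parry montage from the character WeaponComponent's shield data asset.
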(event EventBeginPlay
  (bind _asbp_base_character (Utilities|Casting|CastToBP_BaseCharacter (Components|GetOwner)))
  (Variables|Default|SetOwnerCharacter _asbp_base_character)
  (for (_array_element _array_index) (Rendering|Material|GetMaterials (Variables|Default|GetMesh))
    (bind _returnvalue (Rendering|Material|CreateDynamicMaterialInstance _array_element "None" "None" :!class /Script/Engine.KismetMaterialLibrary))
    (Rendering|Material|SetMaterial (Variables|Default|GetMesh) _array_index _returnvalue)))

(fn ConstructionScript)

(fn AttachShield
  (params (타깃 :type Actor%20Object%20Reference) (SocketName :type Name))
  (Transformation|AttachComponentToComponent 타깃 (Variables|/Script/Engine.Character|GetMesh (Variables|Default|GetOwnerCharacter)) SocketName "KeepRelative" "KeepRelative" "KeepRelative" true))

(fn ColoronOff
  (params (On/Off :type Boolean))
  (bind _as머티리얼_인스턴스_다이내믹 (Utilities|Casting|CastToMaterialInstanceDynamic (Rendering|Material|GetMaterial (Variables|Default|GetMesh) 0)))
  (if On/Off
    (Rendering|Material|SetVectorParameterValue _as머티리얼_인스턴스_다이내믹 "Color" "(R=10.000000,G=5.000000,B=10.000000,A=1.000000)" :!class /Script/Engine.MaterialInstanceDynamic)
    (else
      (Rendering|Material|SetVectorParameterValue _as머티리얼_인스턴스_다이내믹 "Color" "(R=1.000000,G=1.000000,B=1.000000,A=1.000000)" :!class /Script/Engine.MaterialInstanceDynamic))))

(fn CounterParryActivate
  (bind _ownercharacter (Variables|Default|GetOwnerCharacter))
  (bind _weaponcomponent (Variables|/Game/BP/Character/BP_BaseCharacter.BP_BaseCharacter_C|GetWeaponComponent _ownercharacter))
  (bind _shielddataasset (Variables|/Game/BP/Component/BP_WeaponComponent.BP_WeaponComponent_C|GetShieldDataAsset _weaponcomponent))
  (bind _parryanimset (Variables|/Game/BP/DataAsset/Weapon_DataAsset/BP_ShieldDataAsset.BP_ShieldDataAsset_C|GetParryAnimSet _shielddataasset))
  (Animation|PlayAnimMontage _ownercharacter (.parrymontage _parryanimset) (.playrate _parryanimset) "None"))
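; Actor component that holds a character's runtime status, currently handling HP, for a BP_BaseCharacter owner.
; On BeginPlay it caches the owner and copies the Status struct from the StatusDataAsset on that owner's StatusComponent.
; ChangeStatus switches on status type and adds deltas to HP current and max without clamping.
; PrintStatus prints the HP values to screen for debugging.
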(event EventBeginPlay
  (CallFunction|Initialze))

(fn Initialze
  (bind _asbp_base_character (Utilities|Casting|CastToBP_BaseCharacter (Components|GetOwner)))
  (bind _output_get (Variables|Default|SetOwnerCharacter _asbp_base_character))
  (if (and (Utilities|IsValid (Variables|/Game/BP/Character/BP_BaseCharacter.BP_BaseCharacter_C|GetStatusComponent _output_get)) (Utilities|IsValid (Variables|BP_StatusComponent_C|GetStatusDataAsset (Variables|/Game/BP/Character/BP_BaseCharacter.BP_BaseCharacter_C|GetStatusComponent _output_get))))
    (bind _output_get_2 (Variables|Current|SetCurrentStausDataAsset (Variables|BP_StatusComponent_C|GetStatusDataAsset (Variables|/Game/BP/Character/BP_BaseCharacter.BP_BaseCharacter_C|GetStatusComponent _output_get))))
    (Variables|Current|SetCurrentStauts (Variables|/Game/BP/Component/DataAsset/BP_StatusData.BP_StatusData_C|GetStatus _output_get_2))))

(fn PrintStatus
  (params (Type :type E_StatusType%20Enum :default "NewEnumerator2"))
  (bind _currentstauts (Variables|Current|GetCurrentStauts))
  (bind (_current _max) (Utilities|Struct|BreakF_Stat (.hp _currentstauts)))
  (switch Utilities|FlowControl|Switch|SwitchonE_StatusType Type
    (:NewEnumerator2
      (Development|PrintString "Hello"))
    (:NewEnumerator0
      (Development|PrintString (Utilities|String|ToString(Float) _current))
      (Development|PrintString (Utilities|String|ToString(Float) _max)))))

(fn ChangeStatus
  (params (In%20Status%20Type :type E_StatusType%20Enum :default "NewEnumerator2") (InCurrent :type Float%20%28double-precision%29) (In%20Max :type Float%20%28double-precision%29))
  (switch Utilities|FlowControl|Switch|SwitchonE_StatusType In%20Status%20Type
    (:NewEnumerator0
      (Variables|Current|SetCurrentStauts (Utilities|Struct|MakeF_Status (Utilities|Struct|MakeF_Stat (+ (.current (Utilities|Struct|BreakF_Status (Variables|Current|GetCurrentStauts))) InCurrent) (+ (.max (Utilities|Struct|BreakF_Status (Variables|Current|GetCurrentStauts))) In%20Max)))))))
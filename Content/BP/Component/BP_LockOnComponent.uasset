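; BP_LockOnComponent gives a character a toggleable lock-on to a target BP_BaseCharacter.
; Toggling on sphere-traces for pawns along the BP_Player camera's forward vector, starting at the owner, with debug drawing enabled.
; A found target switches the owner from movement-oriented rotation to controller yaw, and toggling off restores this.
; While locked, Tick snaps control rotation from Cam toward the target.
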(event EventBeginPlay
  (bind _asbp_base_character (Utilities|Casting|CastToBP_BaseCharacter (Components|GetOwner)))
  (Variables|Default|SetOwnerCharacter _asbp_base_character))

(event EventTick
  (params (DeltaSeconds :type Float%20%28single-precision%29))
  (bind _cam (Variables|Default|GetCam))
  (if (Variables|Default|GetIsLockOn)
    (Utilities|IsValid (Variables|Default|GetLookAtCharacter)
      (:Is%20Valid
        (if (Utilities|IsValid _cam)
          (Pawn|SetControlRotation (Pawn|GetController (Variables|Default|GetOwnerCharacter)) (Math|Rotator|FindLookatRotation (Transformation|GetWorldLocation _cam) (Transformation|GetActorLocation (Variables|Default|GetLookAtCharacter)))))))))

(fn LockonPlayer
  (bind _ownercharacter (Variables|Default|GetOwnerCharacter))
  (bind _charactermovement (Variables|/Script/Engine.Character|GetCharacterMovement _ownercharacter))
  (if (Variables|Default|GetIsLockOn)
    (Variables|Default|SetLookAtCharacter 0)
    (Variables|Default|SetIsLockOn false)
    (Variables|/Script/Engine.CharacterMovementComponent|SetbOrientRotationToMovement _charactermovement true)
    (Variables|/Script/Engine.Pawn|SetbUseControllerRotationYaw _ownercharacter false)
    (else
      (CallFunction|SetLockonEnemy)
      (Utilities|IsValid (Variables|Default|GetLookAtCharacter)
        (:Is%20Valid
          (Variables|Default|SetIsLockOn true)
          (Variables|/Script/Engine.CharacterMovementComponent|SetbOrientRotationToMovement _charactermovement false)
          (Variables|/Script/Engine.Pawn|SetbUseControllerRotationYaw _ownercharacter true))))))

(fn SetLockonEnemy
  (bind _ownercharacter (Variables|Default|GetOwnerCharacter))
  (bind _returnvalue (Transformation|GetActorLocation _ownercharacter))
  (bind _outhit (Collision|SphereTraceForObjects _returnvalue (+ _returnvalue (* (Math|Vector|GetForwardVector (Transformation|GetWorldRotation (Variables|/Game/BP/Character/Player/BP_Player.BP_Player_C|GetCamera (.AsBP%20Player (Utilities|Casting|CastToBP_Player _ownercharacter))))) (Variables|Default|GetLockOn%20Lenght))) (Variables|Default|GetRadius) (Utilities|Array|MakeArray "ObjectTypeQuery3") false (Utilities|Array|MakeArray (Variables|Default|GetOwnerCharacter)) "ForDuration"))
  (if (.bBlockingHit (Collision|BreakHitResult _outhit))
    (Variables|Default|SetLookAtCharacter (.AsBP%20Base%20Character (Utilities|Casting|CastToBP_BaseCharacter (.HitActor (Collision|BreakHitResult _outhit)))))))